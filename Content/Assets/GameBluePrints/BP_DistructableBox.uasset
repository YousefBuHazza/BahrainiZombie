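; BP_DistructableBox is a box that reacts when a component tagged HeadCollider overlaps its bottom collider, with no destruction logic in these graphs.
; The construction script creates a dynamic material instance on the box mesh for runtime colour changes.
; On a hit, the box turns blue while the UpAndDown timeline drives its relative height and yaw spin, then turns red when the timeline finishes.
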(event OnComponentBeginOverlap(BottomCollider)
  (params (OverlappedComponent :type Primitive%20Component%20Object%20Reference) (OtherActor :type Actor%20Object%20Reference) (OtherComp :type Primitive%20Component%20Object%20Reference) (OtherBodyIndex :type Integer) (bFromSweep :type Boolean) (SweepResult :type Hit%20Result%20Structure%20%28by%20ref%29))
  (bind _box (Variables|Default|GetBox))
  (if (Components|ComponentHasTag OtherComp "HeadCollider")
    (Rendering|Material|SetVectorParameterValue (Variables|Default|GetBoxMaterial) "Box Color" "(R=0.064557,G=0.057000,B=0.848958,A=1.000000)" :!class /Script/Engine.MaterialInstanceDynamic)
    (bind (_direction _upraise _spin) (Timeline|UpAndDown PlayFromStart)
      (:Update
        (Transformation|SetRelativeLocation _box (Math|Vector|MakeVector 0.0 0.0 _upraise) false false)
        (Transformation|SetRelativeRotation _box (Math|Rotator|MakeRotator 0.0 0.0 _spin) false false))
      (:Finished
        (Rendering|Material|SetVectorParameterValue (Variables|Default|GetBoxMaterial) "Box Color" "(R=0.713542,G=0.000000,B=0.124564,A=0.000000)" :!class /Script/Engine.MaterialInstanceDynamic)))))

(event EventBeginPlay)

(event Collision|EventActorBeginOverlap
  (params (OtherActor :type Actor%20Object%20Reference)))

(event EventTick
  (params (DeltaSeconds :type Float%20%28single-precision%29)))

(fn ConstructionScript
  (bind _returnvalue (Rendering|Material|CreateDynamicMaterialInstance (Variables|Default|GetBox) 0 "/Game/Assets/Material/MAT_Box_Inst.MAT_Box_Inst" :!class /Script/Engine.PrimitiveComponent))
  (Variables|Default|SetBoxMaterial _returnvalue))